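; Elevator actor that lifts its Mover component to a height derived from MaxFloors and builds its own shaft walls.
; The construction script sets MaxHeight and places instanced walls for three hardcoded floor levels, omitting the back at MaxFloors and the front at ground level.
; Interact input, enabled while FirstPersonCharacter overlaps the Collider, or PlayerWantstoInteract plays a timeline driving Mover Z.
; Play rate scales ElevatorVelocity by MaxHeight, and leaving the Collider reverses the ride.
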(event `/Game/Blueprints/Interfaces/PlayerCanInteract.Player Wants to Interact`
  (params (Player :type "/Game/Blueprints/FirstPersonCharacter Object Reference"))
  (bind (_direction _percent) (`Timeline|AnimElevate` :!label _label)
    (:`Update`
      (`SceneComponent.K2_SetRelativeLocation` (`self.Mover`) (`KismetMathLibrary.MakeVector` 0.0 0.0 (* _percent (`self.Max Height`))) false false))))

(event `InputAction|Interact`
  (params (Key :type "Key Structure"))
  (:`Pressed`
    (goto _label)))

(event `self.Collider.OnComponentBeginOverlap`
  (params (OverlappedComponent :type "PrimitiveComponent Object Reference") (OtherActor :type "Actor Object Reference") (OtherComp :type "PrimitiveComponent Object Reference") (OtherBodyIndex :type Integer) (bFromSweep :type Boolean) (SweepResult :type "HitResult Structure (by ref)"))
  ;[1 1 1] Enable/Disable Player Input
  (cast `/Game/Blueprints/FirstPersonCharacter` OtherActor)
  (`self.EnableInput` (`GameplayStatics.GetPlayerController` 0)))

(event `self.ReceiveBeginPlay`
  (`TimelineComponent.SetPlayRate` (`self.AnimElevate`) (/ (`self.Elevator Velocity`) (`self.Max Height`))))

(event `self.Collider.OnComponentEndOverlap`
  (params (OverlappedComponent :type "PrimitiveComponent Object Reference") (OtherActor :type "Actor Object Reference") (OtherComp :type "PrimitiveComponent Object Reference") (OtherBodyIndex :type Integer))
  ;[1 1 1] Enable/Disable Player Input
  (cast `/Game/Blueprints/FirstPersonCharacter` OtherActor)
  (`self.DisableInput` (`GameplayStatics.GetPlayerController` 0))
  (goto _label :!via `Reverse`))

(fn `UserConstructionScript`
  (set `self.Max Height` (`KismetMathLibrary.Conv_IntToDouble` (* (`self.Max_Floors`) 400)))
  (for _index (range 3)
    (bind _output_get (set `self.Current_Floor` _index))
    (set `self.Current_z` (* _output_get 400.0))
    ;[1 1 1] Right Wall
    (`InstancedStaticMeshComponent.AddInstance` (`self.Wall Instance Mesh`) (`KismetMathLibrary.MakeTransform` (`KismetMathLibrary.MakeVector` -200.0 210.0 (`self.Current_z`))))
    ;[1 1 1] Left Wall
    (`InstancedStaticMeshComponent.AddInstance` (`self.Wall Instance Mesh`) (`KismetMathLibrary.MakeTransform` (`KismetMathLibrary.MakeVector` -200.0 -210.0 (`self.Current_z`))))
    ;[1 1 1] Back Wall
    (if (!= (`self.Current_Floor`) (`self.Max_Floors`))
      (`InstancedStaticMeshComponent.AddInstance` (`self.Wall Instance Mesh`) (`KismetMathLibrary.MakeTransform` (`KismetMathLibrary.MakeVector` 210.0 -200.0 (`self.Current_z`)) (struct :`Yaw` 90.0))))
    ;[1 1 1] Front Wall
    (if (!= (`self.Current_Floor`) 0)
      (`InstancedStaticMeshComponent.AddInstance` (`self.Wall Instance Mesh`) (`KismetMathLibrary.MakeTransform` (`KismetMathLibrary.MakeVector` -210.0 -200.0 (`self.Current_z`)) (struct :`Yaw` 90.0))))))