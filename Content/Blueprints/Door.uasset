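; Interactive swinging door with a separate lock button, both operated by the Interact input.
; Overlaps of the door and button colliders with the first-person character toggle player input and set AtDoor or AtButton.
; At the door, Interact plays or reverses timelines that scale DoorRotate's yaw up to MaxOpen, provided it is unlocked.
; At the button, Interact toggles the lock and updates the DoorState text.
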(event `InputAction|Interact`
  (params (Key :type "Key Structure"))
  ;[1 1 1] Open and Close Door
  (:`Pressed`
    (if (and (`self.atDoor`) (`self.isClosed`) (`self.isUnlocked`))
      (bind (_direction _percent) (`Timeline|Timeline_1`)
        (:`Update`
          (`SceneComponent.K2_SetRelativeRotation` (`self.Door_Rotate`) (`KismetMathLibrary.MakeRotator` 0.0 0.0 (* _percent (`self.MaxOpen`))) false false)
          (set `self.isClosed` false)))
      (elif (and (`self.atDoor`) (`self.isUnlocked`))
        (if (not (`self.isClosed`))
          (bind (_direction_2 _percent_2) (`Timeline|Timeline_2` :!via `ReverseFromEnd`)
            (:`Update`
              (`SceneComponent.K2_SetRelativeRotation` (`self.Door_Rotate`) (`KismetMathLibrary.MakeRotator` 0.0 0.0 (* _percent_2 (`self.MaxOpen`))) false false)
              (set `self.isClosed` true))))))))

(event `self.Door Collider.OnComponentBeginOverlap`
  (params (OverlappedComponent :type "PrimitiveComponent Object Reference") (OtherActor :type "Actor Object Reference") (OtherComp :type "PrimitiveComponent Object Reference") (OtherBodyIndex :type Integer) (bFromSweep :type Boolean) (SweepResult :type "HitResult Structure (by ref)"))
  ;[1 1 1] Enable/Disable Player Input on Door
  (cast `/Game/Blueprints/FirstPersonCharacter` OtherActor)
  (`self.EnableInput` (`GameplayStatics.GetPlayerController` 0))
  (set `self.atDoor` true))

(event `self.Door Collider.OnComponentEndOverlap`
  (params (OverlappedComponent :type "PrimitiveComponent Object Reference") (OtherActor :type "Actor Object Reference") (OtherComp :type "PrimitiveComponent Object Reference") (OtherBodyIndex :type Integer))
  ;[1 1 1] Enable/Disable Player Input on Door
  (cast `/Game/Blueprints/FirstPersonCharacter` OtherActor)
  (`self.DisableInput` (`GameplayStatics.GetPlayerController` 0))
  (set `self.atDoor` false))

(event `InputAction|Interact`
  (params (Key :type "Key Structure"))
  ;[1 1 1] Lock and Unlock Door
  (:`Pressed`
    (if (`self.atButton`)
      (if (`self.isUnlocked`)
        (`TextRenderComponent.K2_SetText` (`self.DoorState`) (`KismetTextLibrary.Conv_StringToText` "Locked"))
        (set `self.isUnlocked` false)
        (else
          (`TextRenderComponent.K2_SetText` (`self.DoorState`) (`KismetTextLibrary.Conv_StringToText` "Unlocked"))
          (set `self.isUnlocked` true))))))

(event `self.Button_Collider.OnComponentBeginOverlap`
  (params (OverlappedComponent :type "PrimitiveComponent Object Reference") (OtherActor :type "Actor Object Reference") (OtherComp :type "PrimitiveComponent Object Reference") (OtherBodyIndex :type Integer) (bFromSweep :type Boolean) (SweepResult :type "HitResult Structure (by ref)"))
  ;[1 1 1] Enable/Disable Player Input on Button
  (cast `/Game/Blueprints/FirstPersonCharacter` OtherActor)
  (`self.EnableInput` (`GameplayStatics.GetPlayerController` 0))
  (set `self.atButton` true))

(event `self.Button_Collider.OnComponentEndOverlap`
  (params (OverlappedComponent :type "PrimitiveComponent Object Reference") (OtherActor :type "Actor Object Reference") (OtherComp :type "PrimitiveComponent Object Reference") (OtherBodyIndex :type Integer))
  ;[1 1 1] Enable/Disable Player Input on Button
  (cast `/Game/Blueprints/FirstPersonCharacter` OtherActor)
  (`self.DisableInput` (`GameplayStatics.GetPlayerController` 0))
  (set `self.atButton` false))

(fn `UserConstructionScript`)